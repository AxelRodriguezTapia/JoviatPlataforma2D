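; Moving platform for a 2D platformer that shuttles back and forth along the world Y axis.
; BeginPlay stores the starting Y, then each Tick shifts the actor by Speed in the current Direction.
; Once the distance from the stored Y reaches AmplitudMovimiento, Direction flips and that Y becomes the new reference.
; Movement is per frame, not scaled by delta time, so its speed depends on frame rate.
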(event EventBeginPlay
  (Variables|Default|SetPosInit (.y (Transformation|GetActorLocation))))

(event Collision|EventActorBeginOverlap
  (params (OtherActor :type Actor%20Object%20Reference)))

(event EventTick
  (params (DeltaSeconds :type Float%20%28single-precision%29))
  (bind _returnvalue (Transformation|GetActorLocation))
  (bind _returnvalue_2 (Transformation|GetActorLocation))
  (if (Variables|Default|GetDirection)
    (Transformation|SetActorLocation (Math|Vector|MakeVector (.x _returnvalue_2) (+ (.y _returnvalue_2) (Variables|Default|GetSpeed)) (.z _returnvalue_2)) false false)
    (if (> (Variables|Default|GetAmplitudMovimiento) (Math|Float|Absolute(Float) (- (Variables|Default|GetPosInit) (.y _returnvalue_2))))
      (Variables|Default|SetDirection true)
      (else
        (Variables|Default|SetDirection false)
        (Variables|Default|SetPosInit (.y (Transformation|GetActorLocation)))))
    (else
      (Transformation|SetActorLocation (Math|Vector|MakeVector (.x _returnvalue) (- (.y _returnvalue) (Variables|Default|GetSpeed)) (.z _returnvalue)) false false)
      (if (> (Variables|Default|GetAmplitudMovimiento) (Math|Float|Absolute(Float) (- (Variables|Default|GetPosInit) (.y _returnvalue))))
        (Variables|Default|SetDirection false)
        (else
          (Variables|Default|SetDirection true)
          (Variables|Default|SetPosInit (.y (Transformation|GetActorLocation))))))))

(fn ConstructionScript)