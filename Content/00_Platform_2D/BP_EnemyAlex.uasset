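; BP_EnemyAlex is an enemy for the 2D platformer that fires repeatedly and dies from a single bullet hit.
; Tick spawns a BP_EnemyBullet at the Scene component's transform, using the CanFire flag and a DelayFire wait to space shots.
; Overlap of its Box with a BP_Bullet destroys both the bullet and the enemy.
; NewFunction, a spawn helper taking a rotation, is not called within this Blueprint.
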(event OnComponentBeginOverlap(Box)
  (params (OverlappedComponent :type Primitive%20Component%20Object%20Reference) (OtherActor :type Actor%20Object%20Reference) (OtherComp :type Primitive%20Component%20Object%20Reference) (OtherBodyIndex :type Integer) (bFromSweep :type Boolean) (SweepResult :type Hit%20Result%20Structure%20%28by%20ref%29))
  (bind _asbp_bullet (Utilities|Casting|CastToBP_Bullet OtherActor))
  (Actor|DestroyActor _asbp_bullet)
  (Actor|DestroyActor))

(event EventBeginPlay)

(event EventTick
  (params (DeltaSeconds :type Float%20%28single-precision%29))
  (if (Variables|Default|GetCan%20Fire)
    (Variables|Default|SetCan%20Fire false)
    (Game|SpawnActorfromClass "/Game/00_Platform_2D/BP_EnemyBullet.BP_EnemyBullet_C" (Transformation|GetWorldTransform (Variables|Default|GetScene)) "Undefined" "MultiplyWithRoot" 0 0)
    (Utilities|FlowControl|Delay (Variables|Default|GetDelay%20Fire))
    (Variables|Default|SetCan%20Fire true)))

(fn ConstructionScript)

(fn NewFunction
  (params (SpawnTransform_Rotation :type Rotator))
  (Game|SpawnActorfromClass "/Game/00_Platform_2D/BP_EnemyBullet.BP_EnemyBullet_C" (Math|Transform|MakeTransform "0, 0, 0" SpawnTransform_Rotation "1.000000,1.000000,1.000000") "Undefined" "MultiplyWithRoot" 0 0))